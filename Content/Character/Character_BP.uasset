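; Player Character Blueprint with camera-relative movement, mouse look and switchable first/third-person cameras, starting in first person with the body mesh hidden.
; Jog is held while crouch and prone are mutually exclusive FlipFlop toggles, with jog and crouch setting walk speed.
; Prone disables movement and jumping until a short delay after standing.
; Jump is blocked when crouched unless jogging, and its Z velocity varies between moving and stationary.
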(event EventBeginPlay)

(event Collision|EventActorBeginOverlap
  (params (OtherActor :type Actor%20Object%20Reference)))

(event EventTick
  (params (DeltaSeconds :type Float%20%28single-precision%29)))

(event EventBeginPlay
  (Components|Activation|Activate (Variables|Default|GetCamera-1P) false)
  (Rendering|SetVisibility (Variables|Character|GetMesh) false true))

(event Input|ActionEvents|InputActionCameraSwap
  (params (Key :type Key%20Structure))
  (bind _camera_1p (Variables|Default|GetCamera-1P))
  (bind _mesh (Variables|Character|GetMesh))
  (:Pressed
    (Components|Activation|ToggleActive _camera_1p)
    (Components|Activation|ToggleActive (Variables|Default|GetCamera-3P))
    (if (Components|Activation|IsActive _camera_1p)
      (Rendering|SetVisibility _mesh false true)
      (else
        (Rendering|SetVisibility _mesh true true)))))

(event Input|AxisEvents|InputAxisMoveForward
  (params (AxisValue :type Float%20%28single-precision%29))
  (if (not (Variables|Default|GetDisableMovement))
    (Pawn|Input|AddMovementInput (Math|Vector|GetForwardVector (Math|Rotator|MakeRotator 0.0 0.0 (.Yaw (Math|Rotator|BreakRotator (Pawn|GetControlRotation :!class /Script/Engine.Pawn))))) AxisValue false)))

(event Input|AxisEvents|InputAxisMoveRight
  (params (AxisValue :type Float%20%28single-precision%29))
  (if (not (Variables|Default|GetDisableMovement))
    (Pawn|Input|AddMovementInput (Math|Vector|GetRightVector (Math|Rotator|MakeRotator 0.0 0.0 (.Yaw (Math|Rotator|BreakRotator (Pawn|GetControlRotation :!class /Script/Engine.Pawn))))) AxisValue false)))

(event Input|AxisEvents|InputAxisTurn
  (params (AxisValue :type Float%20%28single-precision%29))
  (Pawn|Input|AddControllerYawInput AxisValue))

(event Input|AxisEvents|InputAxisLookUp
  (params (AxisValue :type Float%20%28single-precision%29))
  (Pawn|Input|AddControllerPitchInput AxisValue))

(event Input|ActionEvents|InputActionJog
  (params (Key :type Key%20Structure))
  (bind _charactermovement (Variables|Character|GetCharacterMovement))
  ;[1 1 1] Jog
  (:Pressed
    (Variables|Default|SetJogPressed true)
    (Variables|/Script/Engine.CharacterMovementComponent|SetMaxWalkSpeed _charactermovement 375.0))
  (:Released
    (Variables|Default|SetJogPressed false)
    (if (Variables|Default|GetCrouchPressed)
      (Variables|/Script/Engine.CharacterMovementComponent|SetMaxWalkSpeed _charactermovement 1.6e+02)
      (else
        (Variables|/Script/Engine.CharacterMovementComponent|SetMaxWalkSpeed _charactermovement 2e+02)))))

(event Input|ActionEvents|InputActionCrouch
  (params (Key :type Key%20Structure))
  (bind _charactermovement (Variables|Character|GetCharacterMovement))
  ;[1 1 1] Crouch
  (:Pressed
    (if (not (Variables|Default|GetPronePressed))
      (Utilities|FlowControl|FlipFlop
        (:A
          (Variables|Default|SetCrouchPressed true)
          (Variables|/Script/Engine.CharacterMovementComponent|SetMaxWalkSpeed _charactermovement 1.6e+02))
        (:B
          (Variables|Default|SetCrouchPressed false)
          (if (Variables|Default|GetJogPressed)
            (Variables|/Script/Engine.CharacterMovementComponent|SetMaxWalkSpeed _charactermovement 375.0)
            (else
              (Variables|/Script/Engine.CharacterMovementComponent|SetMaxWalkSpeed _charactermovement 2e+02))))))))

(event Input|ActionEvents|InputActionProne
  (params (Key :type Key%20Structure))
  ;[1 1 1] Prone
  (:Pressed
    (if (not (Variables|Default|GetCrouchPressed))
      (Utilities|FlowControl|FlipFlop
        (:A
          (Variables|Default|SetPronePressed true)
          (Variables|Default|SetDisableMovement true))
        (:B
          (Variables|Default|SetPronePressed false)
          (Utilities|FlowControl|Delay 1.4)
          (Variables|Default|SetDisableMovement false))))))

(event Input|ActionEvents|InputActionJump
  (params (Key :type Key%20Structure))
  (bind _charactermovement (Variables|Character|GetCharacterMovement))
  (:Pressed
    (if (not (Variables|Default|GetDisableMovement))
      (if (Variables|Default|GetCrouchPressed)
        (if (> (Variables|/Script/Engine.CharacterMovementComponent|GetMaxWalkSpeed (Variables|Character|GetCharacterMovement)) 1.6e+02)
          (if (> (Math|Vector|VectorLength (Variables|/Script/Engine.MovementComponent|GetVelocity (Variables|Character|GetCharacterMovement))) 0.0) :!label _label
            (Character|Jump)
            (Variables|/Script/Engine.CharacterMovementComponent|SetJumpZVelocity _charactermovement 365.0)
            (Variables|Default|SetJumpPressed true)
            (else
              (Character|Jump)
              (Variables|/Script/Engine.CharacterMovementComponent|SetJumpZVelocity _charactermovement 3.4e+02)
              (Variables|Default|SetJumpPressed true))))
        (else
          (goto _label)))))
  (:Released
    (Variables|Default|SetJumpPressed false)))

(fn ConstructionScript)