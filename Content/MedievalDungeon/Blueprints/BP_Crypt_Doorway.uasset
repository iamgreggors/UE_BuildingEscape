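; BP_Crypt_Doorway is a crypt double-door actor that swings open on a key press.
; It enables player input at BeginPlay, so F works without any proximity check, hiding the instruction text and playing the DoorSwing timeline.
; The timeline's separate left and right tracks drive each door mesh's yaw in world space, and the construction script presets both doors to a fixed world rotation.
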(event EventBeginPlay
  (Input|EnableInput (Game|GetPlayerController 0)))

(event Collision|EventActorBeginOverlap
  (params (OtherActor :type Actor%20Object%20Reference)))

(event EventTick
  (params (DeltaSeconds :type Float%20%28single-precision%29)))

(event Input|KeyboardEvents|F
  (params (Key :type Key%20Structure))
  (:Pressed
    (Rendering|SetVisibility (Variables|/Script/Engine.TextRenderActor|GetTextRender (Variables|Default|GetTextInstruction)) false false)
    (bind (_direction _doorswing_left _doorswing_right) (Timeline|Door%20Swing Play)
      (:Update
        (Transformation|SetWorldRotation (Variables|Default|GetSM_DoorWay_Large_Door_Left) (Math|Rotator|MakeRotator 0.0 0.0 _doorswing_left) false false)
        (Transformation|SetWorldRotation (Variables|Default|GetSM_DoorWay_Large_Door_Right) (Math|Rotator|MakeRotator 0.0 0.0 _doorswing_right) false false)))))

(fn ConstructionScript
  (Transformation|SetWorldRotation (Variables|Default|GetSM_DoorWay_Large_Door_Left) "0,-90.000000, 0" false false))