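; Dungeon doorway Blueprint with large left and right doors that swing open when the player character class Character_BP overlaps the Trigger_CryptOpen actor.
; BeginPlay resets both doors to zero world rotation.
; The overlap plays the DoorSwing timeline, whose separate left and right tracks set each door's world yaw.
; It has no closing logic, and the rotations are absolute world values, independent of the doorway's placed orientation.
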(event OnActorBeginOverlap(Trigger_CryptOpen)
  (params (OverlappedActor :type Actor%20Object%20Reference) (OtherActor :type Actor%20Object%20Reference))
  (Utilities|Casting|CastToCharacter_BP OtherActor)
  (bind (_direction _doorswing_left _doorswing_right) (Timeline|DoorSwing Play)
    (:Update
      (Transformation|SetWorldRotation (Variables|Default|GetSM_DoorWay_Large_Door_Left) (Math|Rotator|MakeRotator 0.0 0.0 _doorswing_left) false false)
      (Transformation|SetWorldRotation (Variables|Default|GetSM_DoorWay_Large_Door_Right) (Math|Rotator|MakeRotator 0.0 0.0 _doorswing_right) false false))))

(event EventBeginPlay
  (Transformation|SetWorldRotation (Variables|Default|GetSM_DoorWay_Large_Door_Left) (Math|Rotator|MakeRotator 0.0 0.0 0.0) false false)
  (Transformation|SetWorldRotation (Variables|Default|GetSM_DoorWay_Large_Door_Right) (Math|Rotator|MakeRotator 0.0 0.0 0.0) false false))

(event Collision|EventActorBeginOverlap
  (params (OtherActor :type Actor%20Object%20Reference)))

(event EventTick
  (params (DeltaSeconds :type Float%20%28single-precision%29)))

(fn ConstructionScript)