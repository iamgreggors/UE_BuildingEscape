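; Dungeon cell door grate that rises when the gate-raise trigger is overlapped and lowers again when enough mass sits on the exit trigger.
; The RaiseGrate timeline drives the actor's Z, and its completion disables the gate-raise trigger.
; Exit overlap changes re-sum overlapping actors' mass, reversing the timeline at EscapeWeight or above and playing it below.
; Construction sets Z to -400 and disables both triggers' collision.
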(event OnActorBeginOverlap(Trigger_GateRaise)
  (params (OverlappedActor :type Actor%20Object%20Reference) (OtherActor :type Actor%20Object%20Reference))
  (bind _returnvalue (Transformation|GetActorTransform))
  (bind (_location _rotation _scale) (Math|Transform|BreakTransform _returnvalue))
  (bind (_x _y) (Math|Vector|BreakVector _location))
  (if (not (>= (stale OnActorBeginOverlap(Trigger_Exit) _output_get) (Variables|Default|GetEscapeWeight)))
    (bind _gratez_pos (Timeline|RaiseGrate Play)
      (:Update
        (Transformation|SetActorTransform (Math|Transform|MakeTransform (Math|Vector|MakeVector _x _y _gratez_pos) _rotation _scale)))
      (:Finished
        (Collision|SetActorEnableCollision (Variables|Default|GetTrigger_GateRaise) false)))))

(event OnActorBeginOverlap(Trigger_Exit)
  (params (OverlappedActor :type Actor%20Object%20Reference) (OtherActor :type Actor%20Object%20Reference))
  (bind _returnvalue (Transformation|GetActorTransform))
  (bind (_location _rotation _scale) (Math|Transform|BreakTransform _returnvalue))
  (bind (_x _y) (Math|Vector|BreakVector _location))
  (Variables|Default|SetWeightSum 0.0)
  (for _array_element (Collision|GetOverlappingActors (Variables|Default|GetTrigger_Exit) 0 :!class /Script/Engine.Actor)
    (bind _output_get (Variables|Default|SetWeightSum (+ (Variables|Default|GetWeightSum) (Physics|GetMass (Actor|GetComponentbyClass _array_element "/Script/Engine.PrimitiveComponent"))))))
  (if (>= _output_get (Variables|Default|GetEscapeWeight))
    (bind _gratez_pos (Timeline|RaiseGrate Reverse)
      (:Update
        (Transformation|SetActorTransform (Math|Transform|MakeTransform (Math|Vector|MakeVector _x _y _gratez_pos) _rotation _scale)))
      (:Finished
        (Collision|SetActorEnableCollision (Variables|Default|GetTrigger_GateRaise) false)))
    (else
      (Timeline|RaiseGrate Play))))

(event OnActorEndOverlap(Trigger_Exit)
  (params (OverlappedActor :type Actor%20Object%20Reference) (OtherActor :type Actor%20Object%20Reference))
  (bind _returnvalue (Transformation|GetActorTransform))
  (bind (_location _rotation _scale) (Math|Transform|BreakTransform _returnvalue))
  (bind (_x _y) (Math|Vector|BreakVector _location))
  (Variables|Default|SetWeightSum 0.0)
  (for _array_element (Collision|GetOverlappingActors (Variables|Default|GetTrigger_Exit) 0 :!class /Script/Engine.Actor)
    (bind _output_get (Variables|Default|SetWeightSum (+ (Variables|Default|GetWeightSum) (Physics|GetMass (Actor|GetComponentbyClass _array_element "/Script/Engine.PrimitiveComponent"))))))
  (if (>= _output_get (Variables|Default|GetEscapeWeight))
    (bind _gratez_pos (Timeline|RaiseGrate Reverse)
      (:Update
        (Transformation|SetActorTransform (Math|Transform|MakeTransform (Math|Vector|MakeVector _x _y _gratez_pos) _rotation _scale)))
      (:Finished
        (Collision|SetActorEnableCollision (Variables|Default|GetTrigger_GateRaise) false)))
    (else
      (Timeline|RaiseGrate Play))))

(event EventBeginPlay)

(event Collision|EventActorBeginOverlap
  (params (OtherActor :type Actor%20Object%20Reference)))

(fn ConstructionScript
  (bind _returnvalue (Transformation|GetActorTransform))
  (bind (_location _rotation _scale) (Math|Transform|BreakTransform _returnvalue))
  (bind (_x _y) (Math|Vector|BreakVector _location))
  (Transformation|SetActorTransform (Math|Transform|MakeTransform (Math|Vector|MakeVector _x _y -4e+02) _rotation _scale))
  (Collision|SetActorEnableCollision (Variables|Default|GetTrigger_GateRaise) false)
  (Collision|SetActorEnableCollision (Variables|Default|GetTrigger_Exit) false))