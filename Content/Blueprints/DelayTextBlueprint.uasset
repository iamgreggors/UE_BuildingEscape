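; An actor whose TextRender component has its visibility set three seconds after play begins.
; The delayed call shows the text unless the VanishTextOveride flag is set.
; OverrideVanishText sets that flag and hides the text immediately, so a pending delay cannot make it visible again.
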(event EventBeginPlay
  (Utilities|FlowControl|Delay 3.0)
  (Rendering|SetVisibility (Variables|Default|GetTextRender) (not (Variables|Default|GetVanishTextOveride)) false))

(event EventTick
  (params (DeltaSeconds :type Float%20%28single-precision%29)))

(fn ConstructionScript)

(fn OverrideVanishText
  (Variables|Default|SetVanishTextOveride true)
  (Rendering|SetVisibility (Variables|Default|GetTextRender) (not (Variables|Default|GetVanishTextOveride)) false))