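; Win statue actor that signals the win when it reaches the win box.
; The construction script hides the referenced win text and spotlight.
; When WinBoxRef's begin-overlap fires with an actor of exactly the statue's own class, both are made visible.
; The check compares class rather than instance, so any statue of this class triggers the reveal.
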(event OnActorBeginOverlap(WinBoxRef)
  (params (OverlappedActor :type Actor%20Object%20Reference) (OtherActor :type Actor%20Object%20Reference))
  (if (== (Utilities|GetClass OtherActor) (Utilities|GetClass self))
    (Rendering|SetVisibility (Variables|/Script/Engine.TextRenderActor|GetTextRender (Variables|Default|GetWinText)) true false)
    (Rendering|SetVisibility (Variables|/Script/Engine.SpotLight|GetSpotLightComponent (Variables|Default|GetWinSpotRef)) true false)))

(event EventBeginPlay)

(event Collision|EventActorBeginOverlap
  (params (OtherActor :type Actor%20Object%20Reference)))

(event EventTick
  (params (DeltaSeconds :type Float%20%28single-precision%29)))

(fn ConstructionScript
  (Rendering|SetVisibility (Variables|/Script/Engine.TextRenderActor|GetTextRender (Variables|Default|GetWinText)) false false)
  (Rendering|SetVisibility (Variables|/Script/Engine.SpotLight|GetSpotLightComponent (Variables|Default|GetWinSpotRef)) false false))